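; HUD_ToonTanks shows the match-start countdown for Toon Tanks.
; On BeginPlay it adds the W_Start widget to the viewport and switches the player to UI-only input with the mouse locked.
; Tick accumulates time and advances a step counter about once a second, setting the text through a 3-2-1-Start sequence.
; The final step clears the text and restores game-and-UI input, ending the countdown.
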(event EventBeginPlay
  (bind _returnvalue (Game|GetPlayerController 0))
  (bind _returnvalue_2 (UserInterface|CreateWidget "/Game/Blueprints/UI/W_Start.W_Start_C" _returnvalue))
  (bind _output_get (Variables|Default|SetUI _returnvalue_2))
  (UserInterface|Viewport|AddtoViewport _output_get 0)
  (Input|SetInputModeUIOnly _returnvalue 0 "LockAlways" false)
  (Variables|Default|SetStep -1))

(event Collision|EventActorBeginOverlap
  (params (OtherActor :type Actor%20Object%20Reference)))

(event EventTick
  (params (DeltaSeconds :type Float%20%28single-precision%29))
  (bind _ui (Variables|Default|GetUI))
  (bind _starttext (Variables|/Game/Blueprints/UI/W_Start.W_Start_C|GetStartText _ui))
  (Math|Integer|CompareInt (Variables|Default|GetStep) 4
    (:<
      (bind _output_get (Variables|Default|SetTimeElapsed (+ DeltaSeconds (Variables|Default|GetTimeElapsed))))
      (Math|Float|CompareFloat _output_get 1.0
        (:>
          _)
        (:==
          _))
      (bind _result (Math|Integer|IncrementInt (Variables|Default|GetStep))
        (:%20%20
          (Variables|Default|SetTimeElapsed 0.0)
          (switch int _result
            (:Default
              (Variables|/Script/UMG.TextBlock|SetText _starttext (Utilities|Text|MakeLiteralText " ") :!label _label)
              (Input|SetInputModeGameandUI (Game|GetPlayerController 0) 0 "DoNotLock" true false))
            (:0
              (Variables|/Script/UMG.TextBlock|SetText _starttext (Utilities|Text|MakeLiteralText "3")))
            (:1
              (Variables|/Script/UMG.TextBlock|SetText _starttext (Utilities|Text|MakeLiteralText "2")))
            (:2
              (Variables|/Script/UMG.TextBlock|SetText _starttext (Utilities|Text|MakeLiteralText "1")))
            (:3
              (Variables|/Script/UMG.TextBlock|SetText _starttext (Utilities|Text|MakeLiteralText "Start")))
            (:4
              (goto _label))))))))

(fn ConstructionScript)