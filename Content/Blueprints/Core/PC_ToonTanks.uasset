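; Player controller for ToonTanks that points the level's tank at the mouse cursor.
; On BeginPlay it adds the IMC_ToonTanks Enhanced Input mapping context, caches the Tank actor found in the world and shows the cursor.
; Each tick it traces under the cursor on the Visibility channel and passes the hit location to the tank's Aim function.
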(event EventBeginPlay
  (bind _returnvalue (PlayerController|LocalPlayerSubsystems|GetEnhancedInputLocalPlayerSubsystem))
  (Utilities|IsValid _returnvalue
    (:Is%20Valid
      (Input|AddMappingContext _returnvalue "/Game/Blueprints/Inputs/IMC_ToonTanks.IMC_ToonTanks" 0 "(bIgnoreAllPressedKeysUntilRelease=True,bForceImmediately=False,bNotifyUserSettings=False)")
      (bind _returnvalue_2 (Actor|GetActorOfClass "/Script/ToonTanks.Tank"))
      (Variables|Default|SetTank _returnvalue_2)
      (Variables|Default|SetbShowMouseCursor true))))

(event EventTick
  (params (DeltaSeconds :type Float%20%28single-precision%29))
  (bind _tank (Variables|Default|GetTank))
  (if (Utilities|IsValid _tank)
    (Class|Tank|Aim _tank (.Location (Collision|BreakHitResult (.HitResult (Game|Player|GetHitResultUnderCursorbyChannel "TraceTypeQuery1" true)))))))

(fn ConstructionScript)