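; Player-controlled tank that translates input into movement, hull rotation, shooting and aiming.
; Enhanced Input actions drive Move, RotateHull and Shoot, with shots fired from the ShellOrigin component's world location.
; Every tick, it traces under the mouse cursor on the Visibility channel and passes the hit location to Aim.
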(event Input|EnhancedActionEvents|EnhancedInputActionIA_Shoot
  (params (ActionValue :type Boolean) (ElapsedSeconds :type Float%20%28double-precision%29) (TriggeredSeconds :type Float%20%28double-precision%29) (InputAction :type Input%20Action%20Object%20Reference :default "/Game/Blueprints/Inputs/InputActions/IA_Shoot.IA_Shoot"))
  ;[0.8749 0 1] Shoot
  (Class|Tank|Shoot (Transformation|GetWorldLocation (Variables|Components|GetShellOrigin))))

(event Input|EnhancedActionEvents|EnhancedInputActionIA_ForwardBackward
  (params (ActionValue :type Float%20%28double-precision%29) (ElapsedSeconds :type Float%20%28double-precision%29) (TriggeredSeconds :type Float%20%28double-precision%29) (InputAction :type Input%20Action%20Object%20Reference :default "/Game/Blueprints/Inputs/InputActions/IA_ForwardBackward.IA_ForwardBackward"))
  ;[1 0 0] Tank Movement
  (Class|Tank|Move ActionValue))

(event Input|EnhancedActionEvents|EnhancedInputActionIA_RotateLeftRight
  (params (ActionValue :type Float%20%28double-precision%29) (ElapsedSeconds :type Float%20%28double-precision%29) (TriggeredSeconds :type Float%20%28double-precision%29) (InputAction :type Input%20Action%20Object%20Reference :default "/Game/Blueprints/Inputs/InputActions/IA_RotateLeftRight.IA_RotateLeftRight"))
  ;[1 0 0] Tank Movement
  (Class|Tank|RotateHull ActionValue))

(event EventBeginPlay)

(event Collision|EventActorBeginOverlap
  (params (OtherActor :type Actor%20Object%20Reference)))

(event EventTick
  (params (DeltaSeconds :type Float%20%28single-precision%29))
  ;[1 0.9688 0] Aim
  (Class|Tank|Aim (.Location (Collision|BreakHitResult (.HitResult (Game|Player|GetHitResultUnderCursorbyChannel (Game|GetPlayerController 0) "TraceTypeQuery1" true))))))

(fn ConstructionScript)